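; Player controller for boat pawns that forwards throttle, brake and steering input to the possessed boat and drives its control rotation.
; Movement input sets a target pitch and steering sets roll and curve-driven yaw, scaled by speed ratio and, for pitch and yaw, forward/reverse dot product.
; Tick interpolates each rotation axis separately toward that target.
; It also relays dock completion to the HUD.
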(event `self.ReceivePossess`
  (params (PossessedPawn :type "Pawn Object Reference"))
  ;[1 1 1] Update the Current Boat Pawn when we begin and when we change Pawns
  (`parent.ReceivePossess` PossessedPawn)
  (bind _asboat_pawn_base (cast `BoatPawnBase` (`self.K2_GetPawn`) :!label _label))
  (set `self.BoatPawn` (`|ConvertAsset` _asboat_pawn_base))
  (bind _output_get (set `self.TargetControlRotation` (`self.K2_GetActorRotation` _asboat_pawn_base)))
  (`self.SetControlRotation` _output_get))

(event `self.ReceiveBeginPlay`
  ;[1 1 1] Update the Current Boat Pawn when we begin and when we change Pawns
  (goto _label))

(event `self.OnMovementActionTriggered`
  (params (InputActionValue :type "InputActionValue Structure (by ref)"))
  (bind _x (`EnhancedInputLibrary.BreakInputActionValue` InputActionValue))
  (bind (_targetcontrolrotation_roll _targetcontrolrotation_pitch _targetcontrolrotation_yaw) (`KismetMathLibrary.BreakRotator` (`self.TargetControlRotation`)))
  (bind _output (`|ConvertAsset` (`self.BoatPawn`)))
  (`/Engine/EditorBlueprintResources/StandardMacros.IsValid` _output
    (:`Is Valid`
      (if (> _x 0.0)
        (`BoatPawnBase.ThrustForward` _output _x)
        (else
          (`BoatPawnBase.BrakeBoat` _output _x)))
      ;[1 1 1] Rotate the boat upwards slightly when approaching max speed
      (set `self.TargetControlRotation` (`KismetMathLibrary.MakeRotator` _targetcontrolrotation_roll (* (`self.GetBoatSpeedRatio`) (`self.GetBoatDirectionDot`) (`KismetMathLibrary.Lerp` 0.0 (`KismetMathLibrary.FClamp` (+ (.pitch (`self.TargetControlRotation`)) _x) 0.0 10.0) (`KismetMathLibrary.Abs` _x))) _targetcontrolrotation_yaw)))))

(event `EnhancedInput|/Game/Core/Player/Input/IA_Steering`
  (params (ActionValue :type "Float (double-precision)") (ElapsedSeconds :type "Float (double-precision)") (TriggeredSeconds :type "Float (double-precision)") (InputAction :type "InputAction Object Reference" :default "/Game/Core/Player/Input/IA_Steering.IA_Steering"))
  (bind _returnvalue (`self.GetBoatSpeedRatio`))
  (bind _output (`|ConvertAsset` (`self.BoatPawn`)))
  (:`Triggered`
    (`BoatPawnBase.SteerBoat` _output ActionValue)
    (bind _steercurve (`self.SteerCurve` :!label _label_2)
      (:`then`
        (set `self.TargetControlRotation` (`KismetMathLibrary.MakeRotator` (* (`KismetMathLibrary.Lerp` 0.0 (`KismetMathLibrary.FClamp` (+ (.roll (`self.GetControlRotation`)) ActionValue) -10.0 10.0) (`KismetMathLibrary.Abs` ActionValue)) _returnvalue) (.pitch (`self.GetControlRotation`)) (+ (* (`CurveFloat.GetFloatValue` _steercurve ActionValue) _returnvalue (`self.GetBoatDirectionDot`)) (.yaw (`self.GetControlRotation`))))))
      (:`else`)))
  (:`Completed`
    (`BoatPawnBase.SteerBoat` _output 0.0)
    (goto _label_2)))

(event `self.ReceiveTick`
  (params (DeltaSeconds :type "Float (single-precision)"))
  (bind (_returnvalue_roll _returnvalue_pitch _returnvalue_yaw) (`KismetMathLibrary.BreakRotator` (`self.GetControlRotation`)))
  (bind (_targetcontrolrotation_roll _targetcontrolrotation_pitch _targetcontrolrotation_yaw) (`KismetMathLibrary.BreakRotator` (`self.TargetControlRotation`)))
  ;[1 1 1] Rotates the Controlled Boat.
  (`self.SetControlRotation` (`KismetMathLibrary.MakeRotator` (`KismetMathLibrary.FInterpTo` _returnvalue_roll _targetcontrolrotation_roll DeltaSeconds 12.5) (`KismetMathLibrary.FInterpTo` 0.0 _targetcontrolrotation_pitch DeltaSeconds 12.5) (`KismetMathLibrary.FInterpTo` _returnvalue_yaw _targetcontrolrotation_yaw DeltaSeconds 75.0))))

(event `DockTargetInterface.OnDockComplete`
  (message `DockTargetInterface.OnDockComplete` (`self.GetHUD`)))

(fn `GetBoatDirectionDot`
  (returns (ReturnValue :type "Float (double-precision)"))
  (bind _returnvalue (`self.K2_GetPawn`))
  (return (`KismetMathLibrary.Dot_VectorVector` (`KismetMathLibrary.Normal` (`self.GetActorForwardVector` _returnvalue)) (`KismetMathLibrary.Normal` (`self.GetVelocity` _returnvalue)))))

(fn `GetBoatSpeedRatio`
  (returns (ReturnValue :type "Float (double-precision)"))
  (bind _returnvalue (`self.K2_GetPawn`))
  (return (/ (`KismetMathLibrary.VSize` (`self.GetVelocity` _returnvalue)) (`MovementComponent.GetMaxSpeed` (`self.GetComponentByClass` _returnvalue "/Script/Engine.MovementComponent")))))

(fn `UserConstructionScript`)