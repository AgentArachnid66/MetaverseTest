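; Player boat pawn that handles thrust, braking, camera rotation and docking notifications.
; Tick feeds the speed ratio to a Niagara effect and interpolates a scene component toward a height-clamped wave offset for work-in-progress bobbing.
; Thrust and brake apply movement input along the forward vector, with braking limited more tightly at high speed.
; Docking start and completion are relayed to the controller, while SteerBoat is an empty stub.
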(event `self.ReceiveTick`
  (params (DeltaSeconds :type "Float (single-precision)"))
  (bind _scene (`self.Scene`))
  (bind _relativelocation (`SceneComponent.RelativeLocation` _scene))
  (`NiagaraComponent.SetVariableFloat` (`self.Niagara`) "User.NormalisedBoatSpeed" (`self.GetSpeedRatio`))
  ;[1 1 1] Subtle Bobbing motion of the boat. Currently WIP
  (`SceneComponent.K2_SetRelativeLocation` _scene (`KismetMathLibrary.VInterpTo` _relativelocation (`KismetMathLibrary.MakeVector` (.x (+ _relativelocation (`self.GetTargetBoatWaveOffset`))) (.y (+ _relativelocation (`self.GetTargetBoatWaveOffset`))) (`KismetMathLibrary.FClamp` (.z (+ _relativelocation (`self.GetTargetBoatWaveOffset`))) -190.0 -150.0)) DeltaSeconds 50.0) false false))

(event `EnhancedInput|/Game/Core/Player/Input/IA_RotateCamera`
  (params (ActionValue :type "Float (double-precision)") (ElapsedSeconds :type "Float (double-precision)") (TriggeredSeconds :type "Float (double-precision)") (InputAction :type "InputAction Object Reference" :default "/Game/Core/Player/Input/IA_RotateCamera.IA_RotateCamera"))
  (:`Triggered`
    (`SceneComponent.K2_AddRelativeRotation` (`self.SpringArm`) (`KismetMathLibrary.MakeRotator` 0.0 0.0 ActionValue) false false)))

(event `self.BrakeBoat`
  (params (Value :type "Float (single-precision)"))
  (`self.AddMovementInput` (`self.GetActorForwardVector`) (`KismetMathLibrary.FClamp` Value (`KismetMathLibrary.SelectFloat` -1.0 -0.1 (< (`KismetMathLibrary.VSize` (`self.GetVelocity`)) 1000.0)) 0.1)))

(event `self.ThrustForward`
  (params (Value :type "Float (single-precision)"))
  (`self.AddMovementInput` (`self.GetActorForwardVector`) Value))

(event `self.SteerBoat`
  (params (Value :type "Float (single-precision)")))

(event `DockTargetInterface.OnDockStart`
  (`KismetSystemLibrary.PrintText` "Starting to Dock")
  (message `DockTargetInterface.OnDockStart` (`self.GetController`)))

(event `DockTargetInterface.OnDockComplete`
  (`KismetSystemLibrary.PrintText` "Completed Dock")
  (message `DockTargetInterface.OnDockComplete` (`self.GetController`)))

(fn `UserConstructionScript`)